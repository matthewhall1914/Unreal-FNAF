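; Freddy is an enemy AI that roams to random reachable points, pausing between moves.
; Seeing the ThirdPersonCharacter through PawnSensing stops roaming and calls AIMoveTo with that character as the moved Pawn, with no destination set.
; Success plays a sound and attack animation, then reloads the current level.
; Failure waits, returns Freddy to his start location and, on arrival, resumes the roam loop.
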(event `self.ReceiveBeginPlay`
  (bind _returnvalue (`self.K2_GetActorLocation`))
  (set `self.Starting Location` _returnvalue)
  (`|AIMoveTo` self (`NavigationSystemV1.K2_GetRandomReachablePointInRadius` _returnvalue 800.0 null null) null :!label _label
    (:`OnSuccess`
      (`KismetSystemLibrary.Delay` 5.0 :!label _label_2)
      (if (`self.CanRoam`)
        (goto _label)))))

(event `self.PawnSensing.OnSeePawn`
  (params (Pawn :type "Pawn Object Reference"))
  (cast `/Game/ThirdPersonBP/Blueprints/ThirdPersonCharacter` Pawn)
  (set `self.CanRoam` false)
  (`|AIMoveTo` Pawn (0.0 0.0 0.0) null
    (:`OnSuccess`
      (`GameplayStatics.PlaySound2D` "/Game/StarterContent/Audio/Collapse02.Collapse02" 1.0 1.0 0.0 null null)
      (`SkeletalMeshComponent.PlayAnimation` (`self.Mesh`) "/Game/Freddy/FreddyAttack_Anim.FreddyAttack_Anim" false)
      (`KismetSystemLibrary.Delay` 2.0)
      (bind _returnvalue (`GameplayStatics.GetCurrentLevelName` true))
      (`GameplayStatics.OpenLevel` (`KismetStringLibrary.Conv_StringToName` _returnvalue)))
    (:`OnFail`
      (`KismetSystemLibrary.Delay` 5.0)
      (`|AIMoveTo` self (`self.Starting Location`) null
        (:`OnSuccess`
          (set `self.CanRoam` true)
          (goto _label_2))))))

(fn `UserConstructionScript`)